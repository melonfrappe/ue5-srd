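; GassanControllerBP assigns materials to every slot of the referenced Gassan actor's static mesh, creating one dynamic instance of MM_Gassan per slot.
; The Do0-23 event gives the first 24 slots a flat dark green BaseColor.
; The Do24-577 event fills the remaining slots through 577 with textures from the Textures array, matched by slot index offset by 24.
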(event `Do 0-23`
  (for _index (range 24)
    (bind _returnvalue (`KismetMaterialLibrary.CreateDynamicMaterialInstance` "/Game/Materials/MM_Gassan.MM_Gassan"))
    (`MaterialInstanceDynamic.SetVectorParameterValue` _returnvalue "BaseColor" (struct :`R` 0.135505 :`G` 0.252315 :`B` 0.06127 :`A` 1.0))
    (`PrimitiveComponent.SetMaterial` (`StaticMeshActor.StaticMeshComponent` (`self.gassan`)) _index _returnvalue)))

(event `Do 24-577`
  (for _index (range 24 578)
    (bind _returnvalue (`KismetMaterialLibrary.CreateDynamicMaterialInstance` "/Game/Materials/MM_Gassan.MM_Gassan"))
    (`MaterialInstanceDynamic.SetTextureParameterValue` _returnvalue "Texture" (`|GetArrayItem` (`self.textures`) (- _index 24)))
    (`PrimitiveComponent.SetMaterial` (`StaticMeshActor.StaticMeshComponent` (`self.gassan`)) _index _returnvalue)))

(fn `UserConstructionScript`)