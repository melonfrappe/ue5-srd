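; Yachiyoza exterior sequence Blueprint that animates a target actor's transform along a timeline, then switches to the "yachiyoza-inside" level when it finishes.
; It starts after a short delay, and DoMove toggles play and stop, with events for reset, jumping and camera fades.
; Timeline updates report progress to DynamicContextBP, while timeline events spawn 2D audio and toggle Spatial Reality display clipping.
; Tick pauses the audio whenever the timeline is not playing.
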(event `self.ReceiveBeginPlay`
  ;[1 1 1] start
  (`|ExecutionSequence`
    (:`then_0`
      (set `self.defaultTransform` (`self.GetTransform` (`self.target`))))
    (:`then_1`
      (bind _returnvalue (`GameplayStatics.GetActorOfClass` "/Game/Blueprints/DynamicContextBP.DynamicContextBP_C"))
      (set `self.dynamicContext` _returnvalue))
    (:`then_2`
      (`KismetSystemLibrary.Delay` 1.0)
      (`self.Do Move`))))

(event `Set Default`
  ;[1 1 1] reset
  (`self.K2_SetActorTransform` (`self.target`) (`self.defaultTransform`) false false))

(event `Do Move`
  (bind _timeline_backup (`self.Timeline_Backup`))
  ;[1 1 1] move
  (if (`self.isFinished?`)
    (set `self.isFinished?` false)
    (`self.Reset Move`))
  (if (`self.isMove?`)
    (set `self.isMove?` false :!label _label)
    (bind (_direction _location _rotation _scale) (`Timeline|Timeline_Backup` :!via `Stop` :!label _label_2)
      (:`Update`
        (bind _output_get (set `self.currentScale` _scale))
        (`self.K2_SetActorTransform` (`self.target`) (`KismetMathLibrary.MakeTransform` _location (`KismetMathLibrary.MakeRotator` (.x _rotation) (.y _rotation) (.z _rotation)) (`KismetMathLibrary.Conv_DoubleToVector` _output_get)) false false)
        (`/Game/Blueprints/DynamicContextBP.Set Progress` (`self.dynamicContext`) (/ (`TimelineComponent.GetPlaybackPosition` _timeline_backup) (`TimelineComponent.GetTimelineLength` _timeline_backup))))
      (:`Finished`
        (`/Game/Common/SRDisplay/BML_LevelSwitching.SwitchLevel` "yachiyoza-inside"))
      (:`play sound`
        (`self.Play Sound All`))
      (:`toggle clippling`
        (`self.Toggle Clipping`)))
    (else
      (set `self.isMove?` true)
      (goto _label_2))))

(event `Stop Move`
  ;[1 1 1] move
  (goto _label))

(event `Reset Move`
  ;[1 1 1] move
  (goto _label_2 :!via `SetNewTime`))

(event `Play Sound All`
  ;[1 1 1] play
  (bind _returnvalue (`GameplayStatics.SpawnSound2D` (`self.audio_full`) 1.0 1.0 0.0 null))
  (set `self.sound` _returnvalue))

(event `Stop Sound`
  (bind _sound (`self.sound`))
  ;[1 1 1] stop sound
  (`/Engine/EditorBlueprintResources/StandardMacros.IsValid` _sound
    (:`Is Valid`
      (`AudioComponent.Stop` _sound))))

(event `self.ReceiveTick`
  (params (DeltaSeconds :type "Float (single-precision)"))
  (bind _sound (`self.sound`))
  (`/Engine/EditorBlueprintResources/StandardMacros.IsValid` _sound
    (:`Is Valid`
      (`AudioComponent.SetPaused` _sound (not (`TimelineComponent.IsPlaying` (`self.Timeline_Backup`)))))))

(event `Toggle Clipping`
  (bind _srdisplaymanager (`self.srDisplayManager`))
  ;[1 1 1] set clipping
  (set `SRDisplayManager.SpatialClipping` (not (`SRDisplayManager.SpatialClipping` _srdisplaymanager)) _srdisplaymanager))

(event `Jump`
  (params (NewPosition :type "Float (single-precision)"))
  (`TimelineComponent.SetPlaybackPosition` (`self.Timeline_Backup`) NewPosition false true))

(event `Do Fade Camera`
  (params (Duration :type "Float (single-precision)" :default 1.0))
  ;[1 1 1] fade
  (`PlayerCameraManager.StartCameraFade` :`self` (`GameplayStatics.GetPlayerCameraManager` 0) :`ToAlpha` 1.0 :`Duration` 0.5 :`bHoldWhenFinished` true)
  (`KismetSystemLibrary.Delay` Duration)
  (`PlayerCameraManager.StartCameraFade` :`self` (`GameplayStatics.GetPlayerCameraManager` 0) :`FromAlpha` 1.0 :`Duration` 0.5))

(fn `UserConstructionScript`)