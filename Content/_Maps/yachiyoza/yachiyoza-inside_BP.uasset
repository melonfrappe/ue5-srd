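; Drives an automatic, narrated-style camera tour inside the Yachiyoza building, starting one second after BeginPlay.
; Timeline_Camera animates the Target's location, rotation and scale, and reports normalized progress to DynamicContextBP.
; Timeline events switch visible floor meshes, play indexed 2D sounds and trigger a camera fade.
; Play/stop, reset and position jumps control playback; Tick pauses sound with the timeline and shows debug text in non-distribution builds.
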(event `Set Default`
  ;[1 1 1] reset
  (`self.K2_SetActorTransform` (`self.target`) (`self.defaultTransform`) false false))

(event `self.ReceiveBeginPlay`
  ;[1 1 1] start
  (`|ExecutionSequence`
    (:`then_0`
      (set `self.defaultTransform` (`self.GetTransform` (`self.target`))))
    (:`then_1`
      (bind _returnvalue (`GameplayStatics.GetActorOfClass` "/Game/_Blueprints/DynamicContextBP.DynamicContextBP_C"))
      (set `self.dynamicContext` _returnvalue))
    (:`then_2`
      (`KismetSystemLibrary.Delay` 1.0)
      (`self.Do Move`))))

(event `Play Sound Index`
  (params (Index :type Integer))
  ;[1 1 1] play index
  (bind _returnvalue (`GameplayStatics.SpawnSound2D` (`|GetArrayItem` (`self.audios`) Index) 1.0 1.0 0.0 null))
  (set `self.sound` _returnvalue))

(event `Do Move`
  (bind _timeline_camera (`self.Timeline_Camera`))
  ;[1 1 1] Comment
  (if (`self.isFinished?`)
    (`self.Reset Move`))
  (if (`self.isMove?`)
    (set `self.isMove?` false :!label _label)
    (bind (_direction _location _rotation _scale) (`Timeline|Timeline_Camera` :!via `Stop` :!label _label_2)
      (:`Update`
        (bind _output_get (set `self.Scale` _scale))
        (`SceneComponent.K2_SetWorldTransform` (`StaticMeshActor.StaticMeshComponent` (`self.target`)) (`KismetMathLibrary.MakeTransform` _location (`KismetMathLibrary.MakeRotator` (.z _rotation) (.x _rotation) (.y _rotation)) (`KismetMathLibrary.Conv_DoubleToVector` _output_get)) false false)
        (`/Game/_Blueprints/DynamicContextBP.Set Progress` (`self.dynamicContext`) (/ (`TimelineComponent.GetPlaybackPosition` _timeline_camera) (`TimelineComponent.GetTimelineLength` _timeline_camera))))
      (:`Finished`
        (set `self.isFinished?` true)
        (set `self.isMove?` false))
      (:`to 2F`
        (`self.Toggle Floor` 1))
      (:`to 3F`
        (`self.Toggle Floor` 2))
      (:`toggle clipping`)
      (:`play sound 0`
        (`self.Play Sound Index` 0))
      (:`play sound 1`
        (`self.Play Sound Index` 1))
      (:`play sound 2`
        (`self.Play Sound Index` 2))
      (:`play sound 3`
        (`self.Play Sound Index` 3))
      (:`play sound 4`
        (`self.Play Sound Index` 4))
      (:`play sound 5`
        (`self.Play Sound Index` 5))
      (:`play sound 6`
        (`self.Play Sound Index` 6))
      (:`play sound 7`
        (`self.Play Sound Index` 7))
      (:`play sound 8`
        (`self.Play Sound Index` 8))
      (:`play sound 9`
        (`self.Play Sound Index` 9))
      (:`play sound 10`
        (`self.Play Sound Index` 10))
      (:`to base`
        (`self.Do Fade Camera`))
      (:`to 1F`
        (`self.Toggle Floor` 0)))
    (else
      (set `self.isMove?` true)
      (goto _label_2))))

(event `Stop Move`
  ;[1 1 1] Comment
  (goto _label))

(event `Reset Move`
  ;[1 1 1] Comment
  (set `self.isFinished?` false)
  (`self.Toggle Floor` 0)
  (goto _label_2 :!via `SetNewTime`))

(event `Stop Sound`
  (bind _sound (`self.sound`))
  ;[1 1 1] stop sound
  (`/Engine/EditorBlueprintResources/StandardMacros.IsValid` _sound
    (:`Is Valid`
      (`AudioComponent.Stop` _sound))))

(event `Jump Playback Position`
  (params (NewPosition :type "Float (single-precision)"))
  ;[1 1 1] Comment
  (`self.Stop Sound`)
  (`TimelineComponent.SetPlaybackPosition` (`self.Timeline_Camera`) NewPosition false true))

(event `Toggle Floor`
  (params (Index :type Integer))
  (bind _yachiyozameshes (`self.yachiyozaMeshes`))
  ;[1 1 1] delay
  ;;[1 1 1] toggle floor
  (`SceneComponent.SetVisibility` (`StaticMeshActor.StaticMeshComponent` (`|GetArrayItem` _yachiyozameshes Index)) true true)
  (for (_array_element _array_index) _yachiyozameshes
    (`SceneComponent.SetVisibility` (`StaticMeshActor.StaticMeshComponent` _array_element) (== _array_index Index) false)))

(event `Do Fade Camera`
  (`PlayerCameraManager.StartCameraFade` :`self` (`GameplayStatics.GetPlayerCameraManager` 0) :`ToAlpha` 1.0 :`Duration` 0.5 :`bHoldWhenFinished` true)
  (`KismetSystemLibrary.Delay` 1.0)
  (`PlayerCameraManager.StartCameraFade` :`self` (`GameplayStatics.GetPlayerCameraManager` 0) :`FromAlpha` 1.0 :`Duration` 0.5))

(event `Toggle Clipping`
  (bind _srdisplaymanager (`self.srDisplayManager`))
  ;[1 1 1] set clipping
  (set `SRDisplayManager.SpatialClipping` (not (`SRDisplayManager.SpatialClipping` _srdisplaymanager)) _srdisplaymanager))

(event `self.ReceiveTick`
  (params (DeltaSeconds :type "Float (single-precision)"))
  (bind _sound (`self.sound`))
  (`|ExecutionSequence`
    (:`then_0`
      (`/Engine/EditorBlueprintResources/StandardMacros.IsValid` _sound
        (:`Is Valid`
          (`AudioComponent.SetPaused` _sound (not (`TimelineComponent.IsPlaying` (`self.Timeline_Camera`)))))))
    (:`then_1`
      (if (not (`KismetSystemLibrary.IsPackagedForDistribution`))
        (`/Game/_Blueprints/DynamicContextBP.Set Debugger` (`self.dynamicContext`) (`KismetTextLibrary.Conv_TransformToText` (`self.GetTransform` (`self.target`))))
        (`/Game/_Blueprints/DynamicContextBP.SetContext` (`self.dynamicContext`) (`KismetTextLibrary.Conv_StringToText` (`KismetStringLibrary.Concat_StrStr` "再生時間にジャンプするテンキー： \n" "0：最初（1F） \n" "1：断面見る \n" "2：2F \n" "3：ステージ見る \n" "4：地下の通路 \n" "5：天井見る \n")))))))

(fn `UserConstructionScript`)