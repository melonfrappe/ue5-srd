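; DynamicContextBP is a context panel that drives a DynamicContextWidgetBP held in its Widget component, showing a title, description, progress bar and optional image.
; On BeginPlay it pushes its configured text, vertical box width and image settings into the widget and caches the progress bar and debug text.
; Events update title, description, progress and debug text at runtime.
; Debug text updates only outside distribution builds unless DoOverwriteShow is set.
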(event `self.ReceiveBeginPlay`
  (bind _asdynamic_context_widget_bp (cast `/Game/Blueprints/DynamicContextWidgetBP` (`WidgetComponent.GetWidget` (`self.Widget`))))
  (set `/Game/Blueprints/DynamicContextWidgetBP.DescriptionText` (`self.Description`) _asdynamic_context_widget_bp)
  (set `/Game/Blueprints/DynamicContextWidgetBP.TitleText` (`self.Title`) _asdynamic_context_widget_bp)
  (set `self.Progress Bar` (`/Game/Blueprints/DynamicContextWidgetBP.ProgressBar_0` _asdynamic_context_widget_bp))
  (set `self.Debugger` (`/Game/Blueprints/DynamicContextWidgetBP.debugger` _asdynamic_context_widget_bp))
  (`self.Set Vertical Box Sixe X`)
  (`self.Show Image`))

(event `SetDescription`
  (params (Context :type Text))
  (bind _asdynamic_context_widget_bp (cast `/Game/Blueprints/DynamicContextWidgetBP` (`WidgetComponent.GetWidget` (`self.Widget`))))
  (set `/Game/Blueprints/DynamicContextWidgetBP.DescriptionText` Context _asdynamic_context_widget_bp))

(event `Set Title`
  (params (TitleText :type Text))
  (bind _asdynamic_context_widget_bp (cast `/Game/Blueprints/DynamicContextWidgetBP` (`WidgetComponent.GetWidget` (`self.Widget`))))
  (set `/Game/Blueprints/DynamicContextWidgetBP.TitleText` TitleText _asdynamic_context_widget_bp))

(event `Set Progress`
  (params (InPercent :type "Float (double-precision)"))
  (`ProgressBar.SetPercent` (`self.Progress Bar`) InPercent))

(event `Set Debugger`
  (params (InText :type Text))
  (if (or (not (`KismetSystemLibrary.IsPackagedForDistribution`)) (`self.doOverwriteShow?`))
    (`TextBlock.SetText` (`self.Debugger`) (`KismetTextLibrary.Conv_StringToText` (`KismetTextLibrary.Conv_TextToString` InText)))))

(event `Set Vertical Box Sixe X`
  (bind _asdynamic_context_widget_bp (cast `/Game/Blueprints/DynamicContextWidgetBP` (`WidgetComponent.GetWidget` (`self.Widget`))))
  (bind _returnvalue (`WidgetLayoutLibrary.SlotAsCanvasSlot` (`/Game/Blueprints/DynamicContextWidgetBP.VerticalBox_0` _asdynamic_context_widget_bp)))
  (bind (_returnvalue_x _returnvalue_y) (`KismetMathLibrary.BreakVector2D` (`CanvasPanelSlot.GetSize` _returnvalue)))
  (`CanvasPanelSlot.SetSize` _returnvalue (`KismetMathLibrary.MakeVector2D` (`self.In Size X`) _returnvalue_y)))

(event `Show Image`
  (bind _image_visibility (`self.Image Visibility`))
  (bind _asdynamic_context_widget_bp (cast `/Game/Blueprints/DynamicContextWidgetBP` (`WidgetComponent.GetWidget` (`self.Widget`))))
  (set `/Game/Blueprints/DynamicContextWidgetBP.imageVisibility` _image_visibility _asdynamic_context_widget_bp)
  (switch `ESlateVisibility` _image_visibility
    (:`Visible`
      (`CanvasPanelSlot.SetAlignment` (`WidgetLayoutLibrary.SlotAsCanvasSlot` (`/Game/Blueprints/DynamicContextWidgetBP.ScaleBox_0` _asdynamic_context_widget_bp)) (0.0 1.0))
      (bind (_brush_imagesize _brush_margin _brush_tintcolor _brush_outlinesettings _brush_resourceobject) (break `SlateBrush` (`Image.Brush` (`/Game/Blueprints/DynamicContextWidgetBP.Image_0` _asdynamic_context_widget_bp))))
      (`|VariableSetRef` _brush_resourceobject (`self.Image`)))))

(fn `UserConstructionScript`)