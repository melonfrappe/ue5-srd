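; Floating_BP is an actor that shows configurable text on a FloatingWidget_BP hosted in its widget component.
; An Init event casts the widget and applies the InText string, the background image's opacity and the text's vertical alignment within its scale box slot.
; Init runs from both the construction script and BeginPlay, so the settings apply at construction and again when play starts.
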(event `self.ReceiveBeginPlay`
  (`self.Init`))

(event `Init`
  (`self.Set Text`)
  (`self.Set BG Opacity`)
  (`self.Set Alignment`))

(event `Set Text`
  (bind _asfloating_widget_bp (cast `/Game/Blueprints/FloatingWidget_BP` (`WidgetComponent.GetWidget` (`self.Widget`))))
  (`TextBlock.SetText` (`/Game/Blueprints/FloatingWidget_BP.TextBlock` _asfloating_widget_bp) (`self.In Text`)))

(event `Set BG Opacity`
  (bind _asfloating_widget_bp (cast `/Game/Blueprints/FloatingWidget_BP` (`WidgetComponent.GetWidget` (`self.Widget`))))
  (`Image.SetColorAndOpacity` (`/Game/Blueprints/FloatingWidget_BP.Image_BG` _asfloating_widget_bp) (make `LinearColor` 0.0 0.0 0.0 (`self.opacity`))))

(event `Set Alignment`
  (bind _asfloating_widget_bp (cast `/Game/Blueprints/FloatingWidget_BP` (`WidgetComponent.GetWidget` (`self.Widget`))))
  (`ScaleBoxSlot.SetVerticalAlignment` (`WidgetLayoutLibrary.SlotAsScaleBoxSlot` (`/Game/Blueprints/FloatingWidget_BP.TextBlock` _asfloating_widget_bp)) (`self.In Vertical Alignment`)))

(fn `UserConstructionScript`
  (`self.Init`))