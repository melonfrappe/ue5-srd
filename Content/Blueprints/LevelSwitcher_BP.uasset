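; LevelSwitcher_BP switches levels in response to a key passed to its SwitchLevelbyKey event.
; The event selects one of three level maps according to the current entry in the Version list, which names Yoshino and Saigai PLATEAU variants.
; It looks up the key in that map and passes the value to SwitchLevel, doing nothing when the key is absent.
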(event `Switch Level by Key`
  (params (Key :type "Key Structure (by ref)"))
  (bind (_value _returnvalue) (`BlueprintMapLibrary.Map_Find` (`self.Level Map_0`) Key))
  (bind (_value_2 _returnvalue_2) (`BlueprintMapLibrary.Map_Find` (`self.Level Map_1`) Key))
  (bind (_value_3 _returnvalue_3) (`BlueprintMapLibrary.Map_Find` (`self.Level Map_2`) Key))
  (switch `name` (`|GetArrayItem` (`self.version`) (`self.currentVersionIndex`))
    (:`yoshino-saigai-plateau-bim`
      ;[1 1 1] 0
      (if _returnvalue
        (`/Game/Common/SRDisplay/BML_LevelSwitching.SwitchLevel` _value)))
    (:`yoshino-saigai-plateau`
      ;[1 1 1] 1
      (if _returnvalue_2
        (`/Game/Common/SRDisplay/BML_LevelSwitching.SwitchLevel` _value_2)))
    (:`saigai-plateau`
      ;[1 1 1] 2
      (if _returnvalue_3
        (`/Game/Common/SRDisplay/BML_LevelSwitching.SwitchLevel` _value_3)))))

(fn `UserConstructionScript`)