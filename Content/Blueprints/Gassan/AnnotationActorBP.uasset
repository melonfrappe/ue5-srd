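; Annotation label actor that shows a colored text panel in a widget, linked by a cable to a Pivot actor.
; Construction and BeginPlay set the text and colors from variables.
; Tick keeps the label on the Pivot's XY and updates the cable endpoints.
; ToggleHidden hides the label and Pivot's attach parent unless AlwaysShow is set; ToggleShowAnim eases the label's height with a timeline.
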(event `Straighten Label Along Pivot XY`
  (bind _defaultsceneroot (`self.DefaultSceneRoot`))
  (bind (_returnvalue_x _returnvalue_y) (`KismetMathLibrary.BreakVector` (`self.K2_GetActorLocation` (`self.Pivot`))))
  (bind (_returnvalue_x_2 _returnvalue_y_2 _returnvalue_z) (`KismetMathLibrary.BreakVector` (`SceneComponent.K2_GetComponentLocation` _defaultsceneroot)))
  ;[1 1 1] straighten
  (bind _output_get (set `self.defaultLocationZ` _returnvalue_z))
  (`SceneComponent.K2_SetWorldLocation` _defaultsceneroot (`KismetMathLibrary.MakeVector` _returnvalue_x _returnvalue_y _output_get) false false))

(event `self.ReceiveBeginPlay`
  ;[1 1 1] begin play
  (`self.Set Text`)
  (`self.Set Panel Color`)
  (`self.Set Text Color`))

(event `self.ReceiveTick`
  (params (DeltaSeconds :type "Float (single-precision)"))
  ;[1 1 1] tick
  (`/Engine/EditorBlueprintResources/StandardMacros.IsValid` (`self.Pivot`)
    (:`Is Valid`
      (`self.Set Cable Location`)
      (`self.Straighten Label Along Pivot XY`))))

(event `Set Text`
  ;[1 1 1] set text
  (bind _asannotation_widget_bp (cast `/Game/Blueprints/Gassan/AnnotationWidgetBP` (`WidgetComponent.GetWidget` (`self.Widget`))))
  (`TextBlock.SetText` (`/Game/Blueprints/Gassan/AnnotationWidgetBP.TextBlock_1` _asannotation_widget_bp) (`self.In Text`)))

(event `Set Text Color`
  (bind _asannotation_widget_bp (cast `/Game/Blueprints/Gassan/AnnotationWidgetBP` (`WidgetComponent.GetWidget` (`self.Widget`))))
  (`TextBlock.SetColorAndOpacity` (`/Game/Blueprints/Gassan/AnnotationWidgetBP.TextBlock_1` _asannotation_widget_bp) (`self.In Color and Opacity_Text`)))

(event `Set Panel Color`
  (bind _asannotation_widget_bp (cast `/Game/Blueprints/Gassan/AnnotationWidgetBP` (`WidgetComponent.GetWidget` (`self.Widget`))))
  (`Image.SetColorAndOpacity` (`/Game/Blueprints/Gassan/AnnotationWidgetBP.Image_44` _asannotation_widget_bp) (`self.In Color and Opacity_Image`)))

(event `Set Cable Location`
  (bind _cable (`self.Cable`))
  (bind _returnvalue (`SceneComponent.K2_GetComponentLocation` (`self.DefaultSceneRoot`)))
  ;[1 1 1] set cable start/ end point
  (`SceneComponent.K2_SetWorldLocation` _cable (- _returnvalue (0.0 0.0 51.200001)) false false)
  (set `CableComponent.EndLocation` (- (`SceneComponent.K2_GetComponentLocation` (`Actor.RootComponent` (`self.Pivot`))) _returnvalue) _cable))

(event `Toggle Hidden`
  (params (bNewHidden :type Boolean))
  ;[1 1 1] toggle hidden
  (if (not (`self.alwaysShow?`))
    (`SceneComponent.SetHiddenInGame` (`self.DefaultSceneRoot`) bNewHidden true)
    (`self.SetActorHiddenInGame` (`self.GetAttachParentActor` (`self.Pivot`)) bNewHidden)))

(event `Toggle Show Anim`
  (params (`toShow?` :type Boolean))
  (bind (_snapshottransform_x _snapshottransform_y _snapshottransform_z) (`KismetMathLibrary.BreakVector` (`self.snapshotTransform`)))
  (bind (_returnvalue_x _returnvalue_y) (`KismetMathLibrary.BreakVector` (`SceneComponent.K2_GetComponentLocation` (`self.DefaultSceneRoot`))))
  (set `self.snapshotTransform` (`SceneComponent.K2_GetComponentLocation` (`self.DefaultSceneRoot`)))
  (if `toShow?`
    (set `self.bLocationZ` 0.0)
    (bind (_direction _alpha) (`Timeline|Timeline_ToggleShow` :!via `PlayFromStart` :!label _label)
      (:`Update`
        (`SceneComponent.K2_SetWorldLocation` (`self.DefaultSceneRoot`) (`KismetMathLibrary.MakeVector` _returnvalue_x _returnvalue_y (`|EaseFunction` "EaseOut" _alpha _snapshottransform_z (`self.bLocationZ`))) false false)))
    (else
      (set `self.bLocationZ` (`self.defaultLocationZ`))
      (goto _label :!via `PlayFromStart`))))

(fn `UserConstructionScript`
  (`self.Set Text`)
  (`self.Set Panel Color`)
  (`self.Set Text Color`)
  (`self.Set Cable Location`))