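; SplineBP is a construction-time placement actor that repeats a chosen static mesh along a spline.
; The construction script derives spacing from the mesh's bounding-box X size plus an Offset, then fits the instance count to the spline length.
; It adds instances to an InstancedStaticMesh in local space, aligned to the spline at unit scale, with a configurable material.
; The event graph holds no active logic.
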(fn `UserConstructionScript`
  (locals (NumberOfInstances :type Integer :default 0))
  (bind _spline (`self.Spline`))
  (bind _instancedstaticmesh (`self.InstancedStaticMesh`))
  (bind (_min _max) (break `Box` (`StaticMesh.GetBoundingBox` (`self.PlacedMesh`))))
  (`StaticMeshComponent.SetStaticMesh` (`self.InstancedStaticMesh`) (`self.PlacedMesh`))
  (bind _output_get (set `self.Spacing` (+ (.x (- _max _min)) (`self.Offset`))))
  (bind _output_get_2 (set `local.NumberOfInstances` (`KismetMathLibrary.FFloor` (/ (`SplineComponent.GetSplineLength` (`self.Spline`)) _output_get))))
  (for _index (range (+ _output_get_2 1))
    (`PrimitiveComponent.SetMaterial` _instancedstaticmesh 0 (`self.Material`))
    (bind _returnvalue (* _index (`self.Spacing`)))
    (`InstancedStaticMeshComponent.AddInstance` _instancedstaticmesh (`KismetMathLibrary.MakeTransform` (`SplineComponent.GetLocationAtDistanceAlongSpline` _spline _returnvalue "Local") (`SplineComponent.GetRotationAtDistanceAlongSpline` _spline _returnvalue "Local")) false)))