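; Controller Blueprint that shows one glTF model at a time from a list of scene actors and presents its information.
; Visibility is set on static mesh components of each scene actor's recursively attached actors, by index or for the current selection.
; ShowOnlyCurrentIndex also copies the model's GlTF_ComponentBP text into the menu widget.
; Delimited Area matching then toggles map annotations and drives GassanControllerBP's river material for the dam lake.
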(event `Set Model Visibility`
  (params (sceneActor :type "Actor Object Reference") (bNewVisibility :type Boolean))
  (for _array_element (`self.GetAttachedActors` sceneActor true true)
    (for _array_element_2 (`self.K2_GetComponentsByClass` _array_element "/Script/Engine.StaticMeshComponent")
      (`SceneComponent.SetVisibility` _array_element_2 bNewVisibility false))))

(event `Toggle Visibility by Index`
  (params (bNewVisibility :type Boolean) (index :type Integer))
  ;[1 1 1] via runtime
  (`self.Hide All`)
  (bind _output_get (set `self.currentIndex` index))
  (`self.Set Model Visibility` (`|GetArrayItem` (`self.sceneActor`) _output_get) bNewVisibility))

(event `Hide All`
  ;[1 1 1] via editor
  (for _array_element (`self.sceneActor`)
    (`self.Set Model Visibility` _array_element)))

(event `Show Only Current Index`
  ;[1 1 1] via editor
  (`self.Hide All`)
  (`self.Set Model Visibility` (`|GetArrayItem` (`self.sceneActor`) (`self.currentIndex`)) true)
  (`self.Set Prop`))

(event `Set Prop`
  (bind _returnvalue (`self.GetComponentByClass` (`|GetArrayItem` (`self.sceneActor`) (`self.currentIndex`)) "/Game/gltf/Blueprints/glTF_ComponentBP.glTF_ComponentBP_C"))
  (bind _area (`/Game/gltf/Blueprints/glTF_ComponentBP.Area` _returnvalue))
  (bind _returnvalue_2 (`KismetStringLibrary.Concat_StrStr` _area "、"))
  (`/Engine/EditorBlueprintResources/StandardMacros.IsValid` _returnvalue
    (:`Is Valid`
      (bind _returnvalue_3 (`GameplayStatics.GetActorOfClass` "/Game/Blueprints/Gassan/MenuWidgetActorBP.MenuWidgetActorBP_C"))
      (bind _asmenu_widget_bp (cast `/Game/Blueprints/Gassan/MenuWidgetBP` (`WidgetComponent.GetWidget` (`/Game/Blueprints/Gassan/MenuWidgetActorBP.Widget` _returnvalue_3))))
      (`TextBlock.SetText` (`/Game/Blueprints/Gassan/MenuWidgetBP.Title` _asmenu_widget_bp) (`KismetTextLibrary.Conv_StringToText` (`/Game/gltf/Blueprints/glTF_ComponentBP.Title` _returnvalue)))
      (`TextBlock.SetText` (`/Game/Blueprints/Gassan/MenuWidgetBP.Characteristic` _asmenu_widget_bp) (`KismetTextLibrary.Conv_StringToText` (`KismetStringLibrary.Concat_StrStr` "特徴：" (`/Game/gltf/Blueprints/glTF_ComponentBP.Characteristic` _returnvalue))))
      (`TextBlock.SetText` (`/Game/Blueprints/Gassan/MenuWidgetBP.Behaviour` _asmenu_widget_bp) (`KismetTextLibrary.Conv_StringToText` (`KismetStringLibrary.Concat_StrStr` "行動：" (`/Game/gltf/Blueprints/glTF_ComponentBP.Behaviour` _returnvalue))))
      (`TextBlock.SetText` (`/Game/Blueprints/Gassan/MenuWidgetBP.Area` _asmenu_widget_bp) (`KismetTextLibrary.Conv_StringToText` (`KismetStringLibrary.Concat_StrStr` "確認エリア：" _area)))
      ;[1 1 1] all annotation
      (bind _outactors (`GameplayStatics.GetAllActorsOfClass` "/Game/Blueprints/Gassan/AnnotationActorBP.AnnotationActorBP_C"))
      (for _array_element _outactors
        (`/Game/Blueprints/Gassan/AnnotationActorBP.Toggle Hidden` _array_element (not (`KismetStringLibrary.Contains` _returnvalue_2 (`KismetStringLibrary.Concat_StrStr` (`KismetTextLibrary.Conv_TextToString` (`/Game/Blueprints/Gassan/AnnotationActorBP.In Text` _array_element)) "、")))))
      (bind _returnvalue_4 (`GameplayStatics.GetActorOfClass` "/Game/FBX/GassanControllerBP.GassanControllerBP_C"))
      (`/Game/FBX/GassanControllerBP.Do Gassan River Material` _returnvalue_4 (`KismetStringLibrary.Contains` _returnvalue_2 "ダム湖、")))))

(fn `Set glTF Visibility`
  (params (sceneActor1 :type "Actor Object Reference") (bNewVisibility1 :type Boolean)))

(fn `UserConstructionScript`)