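; Controller Blueprint for the Fukuoka Festival glTF models that shows one scene actor at a time from an indexed array.
; Visibility is applied to every static mesh component on actors attached, recursively, to each scene actor.
; ShowOnlyCurrentIndex also copies the model's title, characteristic, behaviour and area from its glTF component into the menu widget.
; ToggleVisibilitybyIndex changes the index and visibility without updating that text.
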(event `Set Model Visibility`
  (params (sceneActor :type "Actor Object Reference") (bNewVisibility :type Boolean))
  (for _array_element (`self.GetAttachedActors` sceneActor true true)
    (for _array_element_2 (`self.K2_GetComponentsByClass` _array_element "/Script/Engine.StaticMeshComponent")
      (`SceneComponent.SetVisibility` _array_element_2 bNewVisibility false))))

(event `Toggle Visibility by Index`
  (params (bNewVisibility :type Boolean) (index :type Integer))
  ;[1 1 1] via runtime
  (`self.Hide All`)
  (bind _output_get (set `self.currentIndex` index))
  (`self.Set Model Visibility` (`|GetArrayItem` (`self.sceneActor`) _output_get) bNewVisibility))

(event `Hide All`
  ;[1 1 1] via editor
  (for _array_element (`self.sceneActor`)
    (`self.Set Model Visibility` _array_element)))

(event `Show Only Current Index`
  ;[1 1 1] via editor
  (`self.Hide All`)
  (`self.Set Model Visibility` (`|GetArrayItem` (`self.sceneActor`) (`self.currentIndex`)) true)
  (`self.Set Prop`))

(event `Set Prop`
  (bind _returnvalue (`self.GetComponentByClass` (`|GetArrayItem` (`self.sceneActor`) (`self.currentIndex`)) "/Game/FukuokaFestival/Blueprints/FukuokaFestival_glTF_ComponentBP.FukuokaFestival_glTF_ComponentBP_C"))
  (`/Engine/EditorBlueprintResources/StandardMacros.IsValid` _returnvalue
    (:`Is Valid`
      (bind _returnvalue_2 (`GameplayStatics.GetActorOfClass` "/Game/FukuokaFestival/Blueprints/FukuokaFestival_MenuWidgetActorBP.FukuokaFestival_MenuWidgetActorBP_C"))
      (bind _asfukuoka_festival_menu_widget_bp (cast `/Game/FukuokaFestival/Blueprints/FukuokaFestival_MenuWidgetBP` (`WidgetComponent.GetWidget` (`/Game/FukuokaFestival/Blueprints/FukuokaFestival_MenuWidgetActorBP.Widget` _returnvalue_2))))
      (`TextBlock.SetText` (`/Game/FukuokaFestival/Blueprints/FukuokaFestival_MenuWidgetBP.Title` _asfukuoka_festival_menu_widget_bp) (`KismetTextLibrary.Conv_StringToText` (`/Game/FukuokaFestival/Blueprints/FukuokaFestival_glTF_ComponentBP.Title` _returnvalue)))
      (`TextBlock.SetText` (`/Game/FukuokaFestival/Blueprints/FukuokaFestival_MenuWidgetBP.Characteristic` _asfukuoka_festival_menu_widget_bp) (`KismetTextLibrary.Conv_StringToText` (`/Game/FukuokaFestival/Blueprints/FukuokaFestival_glTF_ComponentBP.Characteristic` _returnvalue)))
      (`TextBlock.SetText` (`/Game/FukuokaFestival/Blueprints/FukuokaFestival_MenuWidgetBP.Behaviour` _asfukuoka_festival_menu_widget_bp) (`KismetTextLibrary.Conv_StringToText` (`/Game/FukuokaFestival/Blueprints/FukuokaFestival_glTF_ComponentBP.Behaviour` _returnvalue)))
      (`TextBlock.SetText` (`/Game/FukuokaFestival/Blueprints/FukuokaFestival_MenuWidgetBP.Area` _asfukuoka_festival_menu_widget_bp) (`KismetTextLibrary.Conv_StringToText` (`/Game/FukuokaFestival/Blueprints/FukuokaFestival_glTF_ComponentBP.Area` _returnvalue))))))

(fn `Set glTF Visibility`
  (params (sceneActor1 :type "Actor Object Reference") (bNewVisibility1 :type Boolean)))

(fn `UserConstructionScript`)