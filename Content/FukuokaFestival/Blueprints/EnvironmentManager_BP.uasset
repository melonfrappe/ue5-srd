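; EnvironmentManager_BP is an environment controller that toggles the look of the shore and sky in the level.
; ToggleShore flips the visibility of the Shore static mesh and its children, hiding it on the first call.
; ToggleSkyAtmosphereRayleigh alternates the SkyAtmosphere Rayleigh scattering between black and blue.
; ToggleBundle fires both events, each of which keeps its own FlipFlop state.
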(event `Toggle Shore`
  (bind _isa (`/Engine/EditorBlueprintResources/StandardMacros.FlipFlop`)
    (:`A`
      _)
    (:`B`
      _))
  (`SceneComponent.SetVisibility` (`StaticMeshActor.StaticMeshComponent` (`self.Shore`)) (not _isa) true))

(event `Toggle SkyAtmosphere Rayleigh`
  (bind _skyatmospherecomponent (`SkyAtmosphere.SkyAtmosphereComponent` (`self.SkyAtmosphere`)))
  (`/Engine/EditorBlueprintResources/StandardMacros.FlipFlop`
    (:`A`
      (`SkyAtmosphereComponent.SetRayleighScattering` :`self` _skyatmospherecomponent))
    (:`B`
      (`SkyAtmosphereComponent.SetRayleighScattering` _skyatmospherecomponent (struct :`R` 0.174647 :`G` 0.40724 :`B` 1.0 :`A` 1.0)))))

(event `Toggle Bundle`
  (`self.Toggle Shore`)
  (`self.Toggle SkyAtmosphere Rayleigh`))

(fn `UserConstructionScript`)