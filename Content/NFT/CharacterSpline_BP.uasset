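; Spline-following character actor that walks a skeletal character along a path and fires a finished event at the end.
; Play runs a timeline mapped to spline distance, switching from walk to idle at hard-coded spline indices and idling on completion.
; A second timeline eases a mask's scale on play, reset and snap-to-end, while Tick keeps the mask's world rotation at zero.
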(event `Set Animation`
  (bind _spline (`self.Spline`))
  (bind _returnvalue (`KismetMathLibrary.FTrunc` (* (`SplineComponent.GetNumberOfSplinePoints` _spline) (`SplineComponent.GetInputKeyAtDistanceAlongSpline` _spline (`self.DistanceAlongSpline`)))))
  ;[1 1 1] TODO: animation
  (if (!= _returnvalue (`self.currentSplineIndex`))
    (set `self.currentSplineIndex` _returnvalue)
    (if (or (== _returnvalue 9) (== _returnvalue 10))
      (`/Engine/EditorBlueprintResources/StandardMacros.DoOnce` false :!label _label
        (:`Completed`
          (`SkeletalMeshComponent.PlayAnimation` (`self.Character`) "/Game/Characters/Mannequins/Animations/Manny/MM_Idle.MM_Idle" true)
          (goto _label_2 :!via `Reset`)))
      (else
        (`/Engine/EditorBlueprintResources/StandardMacros.DoOnce` false :!label _label_2
          (:`Completed`
            (`SkeletalMeshComponent.PlayAnimation` (`self.Character`) "/Game/Characters/Mannequins/Animations/Manny/MM_Walk_Fwd.MM_Walk_Fwd" true)
            (goto _label :!via `Reset`)))))))

(event `Play`
  (bind _character (`self.Character`))
  (bind _returnvalue (`SplineComponent.GetTransformAtDistanceAlongSpline` (`self.Spline`) (`self.DistanceAlongSpline`) "Local" false))
  (bind _returnvalue_2 (`SplineComponent.GetSplineLength` (`self.Spline`)))
  ;[1 1 1] play
  (`self.Set Mask Size` 20.0)
  (`SceneComponent.SetVisibility` (`self.Character`) true false)
  (`SkeletalMeshComponent.PlayAnimation` (`self.Character`) "/Game/Characters/Mannequins/Animations/Manny/MM_Walk_Fwd.MM_Walk_Fwd" true)
  (`TimelineComponent.SetPlayRate` (`self.Timeline_0`) (`self.newPlayRate`))
  (bind (_direction _alpha) (`Timeline|Timeline_0` :!via `PlayFromStart`)
    (:`Update`
      (`self.Set Animation`)
      (bind _returnvalue_3 (`KismetMathLibrary.Lerp` 0.0 _returnvalue_2 _alpha))
      (if (< _returnvalue_3 _returnvalue_2)
        (set `self.DistanceAlongSpline` _returnvalue_3)
        (`SceneComponent.K2_SetRelativeTransform` _character (`KismetMathLibrary.MakeTransform` (`KismetMathLibrary.MakeVector` (.x (.location _returnvalue)) (.y (.location _returnvalue)) (+ (.z (.location _returnvalue)) 0.0)) (`KismetMathLibrary.MakeRotator` 0.0 0.0 (+ (.yaw (.rotation _returnvalue)) -90.0)) (`SceneComponent.RelativeScale3D` _character)) false false)))
    (:`Finished`
      (`SkeletalMeshComponent.PlayAnimation` (`self.Character`) "/Game/Characters/Mannequins/Animations/Manny/MM_Idle.MM_Idle" true)
      (`self.IsFinished_Event`))))

(event `Set Mask Size`
  (params (`Mask Size` :type "Float (double-precision)" :default 15.0))
  ;[1 1 1] mask
  (set `self.snapshotScale` (`SceneComponent.K2_GetComponentScale` (`self.Mask`)))
  (bind (_direction _alpha) (`Timeline|Timeline_1` :!via `PlayFromStart`)
    (:`Update`
      (`SceneComponent.SetWorldScale3D` (`self.Mask`) (`|EaseFunction` "EaseOut" _alpha (`self.snapshotScale`) (`KismetMathLibrary.Conv_DoubleToVector` `Mask Size`))))))

(event `Reset`
  ;[1 1 1] reset
  (`TimelineComponent.Stop` (`self.Timeline_1`))
  (`TimelineComponent.Stop` (`self.Timeline_0`))
  (set `self.DistanceAlongSpline` 0.0)
  (`SceneComponent.K2_SetRelativeTransform` (`self.Character`) (`KismetMathLibrary.MakeTransform` (0.0 0.0 0.0) (struct :`Yaw` -90.0)) false false)
  (`self.Set Mask Size` 0.1))

(event `Set Last Position`
  (bind _character (`self.Character`))
  (bind _returnvalue (`SplineComponent.GetTransformAtDistanceAlongSpline` (`self.Spline`) (`self.DistanceAlongSpline`) "Local" false))
  ;[1 1 1] set last
  (set `self.DistanceAlongSpline` (`SplineComponent.GetSplineLength` (`self.Spline`)))
  (`SceneComponent.K2_SetRelativeTransform` _character (`KismetMathLibrary.MakeTransform` (`KismetMathLibrary.MakeVector` (.x (.location _returnvalue)) (.y (.location _returnvalue)) (+ (.z (.location _returnvalue)) 0.0)) (`KismetMathLibrary.MakeRotator` 0.0 0.0 (+ (.yaw (.rotation _returnvalue)) -90.0)) (`SceneComponent.RelativeScale3D` _character)) false false)
  (`self.Set Mask Size` 15.0))

(event `self.ReceiveTick`
  (params (DeltaSeconds :type "Float (single-precision)"))
  (`SceneComponent.K2_SetWorldRotation` :`self` (`self.Mask`)))

(fn `UserConstructionScript`)