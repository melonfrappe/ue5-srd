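; Capsule animation Blueprint in the NFT folder that toggles a capsule display between two poses via a custom Play event.
; A FlipFlop alternately plays and reverses one timeline on successive calls.
; The timeline's alpha lerps the Window actor's yaw and the X positions of the Mask and Capsule actors, setting absolute transforms in sync.
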(event `self.ReceiveBeginPlay`
  (`TimelineComponent.SetPlayRate` (`self.Timeline_0`) 1.0))

(event `Play`
  (`/Engine/EditorBlueprintResources/StandardMacros.FlipFlop`
    (:`A`
      (bind (_direction _alpha) (`Timeline|Timeline_0` :!label _label)
        (:`Update`
          (`self.K2_SetActorRotation` (`self.window`) (`KismetMathLibrary.MakeRotator` 0.0 0.0 (`KismetMathLibrary.Lerp` -90.0 -200.0 _alpha)) false)
          (`self.K2_SetActorLocation` (`self.mask`) (`KismetMathLibrary.MakeVector` (`KismetMathLibrary.Lerp` 400.0 200.0 _alpha)) false false)
          (`self.K2_SetActorLocation` (`self.capsule`) (`KismetMathLibrary.MakeVector` (`KismetMathLibrary.Lerp` 0.0 25.0 _alpha)) false false))))
    (:`B`
      (goto _label :!via `Reverse`))))

(fn `UserConstructionScript`)