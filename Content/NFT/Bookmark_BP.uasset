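; Bookmark actor with Pointer and Ground components whose visibility can be toggled as a whole.
; BeginPlay applies the VisibilityOverwrite variable to the root and its children, and the ToggleVisibility event sets it to a passed-in value.
; The construction script gives the Pointer the root's roll and yaw, offsets its pitch by the root's pitch, and resets the Ground to zero world rotation.
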(event `self.ReceiveBeginPlay`
  (`SceneComponent.SetVisibility` (`self.DefaultSceneRoot`) (`self.visibilityOverwrite`) true))

(event `Toggle Visibility`
  (params (bNewVisibility :type Boolean))
  (`SceneComponent.SetVisibility` (`self.DefaultSceneRoot`) bNewVisibility true))

(fn `UserConstructionScript`
  (bind _pointer (`self.Pointer`))
  (bind (_returnvalue_roll _returnvalue_pitch _returnvalue_yaw) (`KismetMathLibrary.BreakRotator` (`SceneComponent.K2_GetComponentRotation` (`self.DefaultSceneRoot`))))
  (bind (_returnvalue_roll_2 _returnvalue_pitch_2) (`KismetMathLibrary.BreakRotator` (`SceneComponent.K2_GetComponentRotation` _pointer)))
  (`SceneComponent.K2_SetWorldRotation` _pointer (`KismetMathLibrary.MakeRotator` _returnvalue_roll (- _returnvalue_pitch_2 _returnvalue_pitch) _returnvalue_yaw) false false)
  (`SceneComponent.K2_SetWorldRotation` (`self.Ground`) (`KismetMathLibrary.MakeRotator` 0.0) false false))