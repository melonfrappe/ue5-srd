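; Tour actor that moves a Target actor to the bookmark at GoIndex when Go is called.
; A timeline alpha drives an ease-out of location and rotation, re-based on the Target's current transform each update.
; For bookmarks with "Elevator" in their name, LiftBody's height follows toward just below the bookmark.
; BeginPlay sets the play rate from NewRate, which also sets an early stop cutoff; alpha is debug-printed.
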(event `self.ReceiveBeginPlay`
  (`|ExecutionSequence`
    (:`then_0`
      (`TimelineComponent.SetPlayRate` (`self.Timeline_0`) (`self.newRate`)))))

(event `Go`
  (bind _target (`self.target`))
  (bind _liftbody (`self.liftBody`))
  (bind (_returnvalue_x _returnvalue_y _returnvalue_z) (`KismetMathLibrary.BreakVector` (`self.K2_GetActorLocation` _liftbody)))
  (bind _output (`|GetArrayItem` (`self.bookmarks`) (`self.goIndex`)))
  (bind (_returnvalue_x_2 _returnvalue_y_2 _returnvalue_z_2) (`KismetMathLibrary.BreakVector` (`self.K2_GetActorLocation` _output)))
  (bind (_direction _alpha) (`Timeline|Timeline_0` :!via `PlayFromStart`)
    (:`Update`
      (bind (_result_location _result_rotation) (`KismetMathLibrary.BreakTransform` (`|EaseFunction` "EaseOut" _alpha (`self.GetTransform` _target) (`self.GetTransform` (`|GetArrayItem` (`self.bookmarks`) (`self.goIndex`))))))
      (`self.K2_SetActorLocationAndRotation` _target _result_location _result_rotation false false)
      (`KismetSystemLibrary.PrintString` (`KismetStringLibrary.Conv_DoubleToString` _alpha))
      (if (`KismetStringLibrary.Contains` (`KismetSystemLibrary.GetDisplayName` _output) "Elevator")
        (`self.K2_SetActorLocation` _liftbody (`KismetMathLibrary.MakeVector` _returnvalue_x _returnvalue_y (`|EaseFunction` "EaseOut" _alpha _returnvalue_z (- _returnvalue_z_2 20.0) 1.8)) false false))
      (if (> (`TimelineComponent.GetPlaybackPosition` (`self.Timeline_0`)) (* (`self.newRate`) 2.0))
        (`TimelineComponent.Stop` (`self.Timeline_0`))))))

(fn `UserConstructionScript`)