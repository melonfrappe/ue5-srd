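; Capsule manager Blueprint that drives the animation of a group of capsule actors attached to CapsuleParent.
; On BeginPlay it gathers the directly attached actors, adds a CapsuleMovement_Component to each with its array index, and caches the DynamicContextBP actor.
; The DoAnimation event calls DoAlpha on every capsule's component, leaving the motion to that component.
; Tick is empty, and the debugger output is disconnected.
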(event `self.ReceiveBeginPlay`
  (`|ExecutionSequence`
    (:`then_0`
      (bind _output_get (set `self.capsules` (`self.GetAttachedActors` (`self.capsuleParent`) true false)))
      (for (_array_element _array_index) _output_get
        (bind _returnvalue (`|AddComponentByClass` _array_element "/Game/NFT/CapsuleMovement_Component.CapsuleMovement_Component_C"))
        (set `/Game/NFT/CapsuleMovement_Component.index` _array_index _returnvalue)))
    (:`then_1`
      (bind _returnvalue_2 (`GameplayStatics.GetActorOfClass` "/Game/_Blueprints/DynamicContextBP.DynamicContextBP_C"))
      (set `self.Dynamic Context` _returnvalue_2))))

(event `Do Animation`
  (for _array_element (`self.capsules`)
    (`/Game/NFT/CapsuleMovement_Component.Do Alpha` (`self.GetComponentByClass` _array_element "/Game/NFT/CapsuleMovement_Component.CapsuleMovement_Component_C"))))

(event `self.ReceiveTick`
  (params (DeltaSeconds :type "Float (single-precision)")))

(fn `UserConstructionScript`)