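; BP_SRDisplayDebugManager is a debug actor for the SR display, built around an FPS text render component.
; The construction script applies a configurable TextColor to that text.
; Tick passes delta time to UpdatePerformance, but that function is empty: the node chain that would write an "FPS:" string is disconnected, so the readout never updates.
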(event `self.ReceiveTick`
  (params (DeltaSeconds :type "Float (single-precision)"))
  (`self.UpdatePerformance` DeltaSeconds))

(fn `UpdatePerformance`
  (params (`Delta Time` :type "Float (double-precision)")))

(fn `UserConstructionScript`
  (`TextRenderComponent.SetTextRenderColor` (`self.FPS`) (`self.TextColor`)))